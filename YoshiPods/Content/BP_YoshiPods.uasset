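; Interactive earbud-case actor that the player spins around its yaw by dragging the left mouse button.
; Clicking the lid opens or closes it, and clicking either head takes out or returns the pods, all animated by Timeline-driven Lerps.
; State flags allow pods out only with the lid open and block closing while they are out.
; Top and bottom part clicks step a Volume variable, and lid hover toggles a HandShow flag.
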(event `self.ReceiveBeginPlay`
  (set `self.PodsOldLocation` (`SceneComponent.RelativeLocation` (`self.Pods`)))
  (`self.EnableInput` (`GameplayStatics.GetPlayerController` 0)))

(event `self.ReceiveTick`
  (params (DeltaSeconds :type "Float (single-precision)"))
  (if (`self.bIsDragging`)
    (bind _output_get (set `self.CurrentMouseX` (`PlayerController.GetMousePosition` (`GameplayStatics.GetPlayerController` 0))))
    (`self.K2_AddActorLocalRotation` (`KismetMathLibrary.MakeRotator` 0.0 0.0 (* (- (`self.LastMouseX`) _output_get) 0.1)))
    (set `self.LastMouseX` (`self.CurrentMouseX`))))

(event `self.Lid.OnClicked`
  (params (TouchedComponent :type "PrimitiveComponent Object Reference") (ButtonPressed :type "Key Structure"))
  (if (`self.bIsLidOpened`)
    (if (not (`self.bIsPodsTaken`))
      (set `self.bIsLidOpened` false)
      (bind (_direction _openalpha) (`Timeline|LidCloseTimeline` :!via `PlayFromStart`)
        (:`Update`
          (`SceneComponent.K2_SetRelativeRotation` (`self.Lid`) (`KismetMathLibrary.MakeRotator` (`KismetMathLibrary.Lerp` -90.0 0.0 _openalpha)) false false))))
    (else
      (set `self.bIsLidOpened` true)
      (bind (_direction_2 _openalpha_2) (`Timeline|LidOpenTimeline` :!via `PlayFromStart`)
        (:`Update`
          (`SceneComponent.K2_SetRelativeRotation` (`self.Lid`) (`KismetMathLibrary.MakeRotator` (`KismetMathLibrary.Lerp` 0.0 90.0 _openalpha_2)) false false))))))

(event `Key|LeftMouseButton`
  (params (Key :type "Key Structure"))
  (:`Pressed`
    (set `self.bIsDragging` true)
    (set `self.LastMouseX` (`PlayerController.GetMousePosition` (`GameplayStatics.GetPlayerController` 0))))
  (:`Released`
    (set `self.bIsDragging` false)))

(event `self.Pods.OnClicked`
  (params (TouchedComponent :type "PrimitiveComponent Object Reference") (ButtonPressed :type "Key Structure")))

(event `self.RightHead.OnClicked`
  (params (TouchedComponent :type "PrimitiveComponent Object Reference") (ButtonPressed :type "Key Structure"))
  (bind (_podsoldlocation_x _podsoldlocation_y _podsoldlocation_z) (`KismetMathLibrary.BreakVector` (`self.PodsOldLocation`)))
  (bind (_podsoldlocation_x_2 _podsoldlocation_y_2 _podsoldlocation_z_2) (`KismetMathLibrary.BreakVector` (`self.PodsOldLocation`)))
  (if (`self.bIsPodsTaken`) :!label _label
    (set `self.bIsPodsTaken` false)
    (bind (_direction _openalpha) (`Timeline|Timeline` :!via `PlayFromStart`)
      (:`Update`
        (`SceneComponent.K2_SetRelativeLocation` (`self.Pods`) (`KismetMathLibrary.MakeVector` 0.0 0.0 (`KismetMathLibrary.Lerp` _podsoldlocation_z_2 (+ _podsoldlocation_z_2 20.0) _openalpha)) false false)))
    (elif (`self.bIsLidOpened`)
      (set `self.bIsPodsTaken` true)
      (bind (_direction_2 _openalpha_2) (`Timeline|PodsTakeOutTimeline` :!via `PlayFromStart`)
        (:`Update`
          (`SceneComponent.K2_SetRelativeLocation` (`self.Pods`) (`KismetMathLibrary.MakeVector` 0.0 0.0 (`KismetMathLibrary.Lerp` _podsoldlocation_z (+ _podsoldlocation_z 20.0) _openalpha_2)) false false))))))

(event `self.LeftHead.OnClicked`
  (params (TouchedComponent :type "PrimitiveComponent Object Reference") (ButtonPressed :type "Key Structure"))
  (goto _label))

(event `self.LeftTop.OnClicked`
  (params (TouchedComponent :type "PrimitiveComponent Object Reference") (ButtonPressed :type "Key Structure"))
  (if (< (`self.Volume`) 1.0) :!label _label_2
    (set `self.Volume` (+ (`self.Volume`) 0.1))))

(event `self.RightTop.OnClicked`
  (params (TouchedComponent :type "PrimitiveComponent Object Reference") (ButtonPressed :type "Key Structure"))
  (goto _label_2))

(event `self.RightBot.OnClicked`
  (params (TouchedComponent :type "PrimitiveComponent Object Reference") (ButtonPressed :type "Key Structure"))
  (if (> (`self.Volume`) 0.0) :!label _label_3
    (set `self.Volume` (- (`self.Volume`) 0.1))))

(event `self.LeftBot.OnClicked`
  (params (TouchedComponent :type "PrimitiveComponent Object Reference") (ButtonPressed :type "Key Structure"))
  (goto _label_3))

(event `self.Lid.OnBeginCursorOver`
  (params (TouchedComponent :type "PrimitiveComponent Object Reference"))
  (set `self.handShow?` true))

(event `self.Lid.OnEndCursorOver`
  (params (TouchedComponent :type "PrimitiveComponent Object Reference"))
  (set `self.handShow?` false))

(fn `UserConstructionScript`)